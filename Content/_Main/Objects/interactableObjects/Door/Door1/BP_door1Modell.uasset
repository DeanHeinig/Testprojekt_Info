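; Interactable door Blueprint that the player can open and close, with its state tracked in DoorStatus.
; Interact flips the state and plays or reverses the DoorMechanics timeline, whose track drives the yaw of DoorMesh's relative rotation.
; ShowInfo passes a German open or close key prompt to the HUD, matching the current state.
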(event EventBeginPlay)

(event Collision|EventActorBeginOverlap
  (params (OtherActor :type Actor%20Object%20Reference)))

(event EventTick
  (params (DeltaSeconds :type Float%20%28single-precision%29)))

(event EventInteract
  (switch Utilities|FlowControl|Switch|SwitchonEN_door-Status (Variables|Default|GetdoorStatus)
    (:NewEnumerator0
      (Variables|Default|SetdoorStatus "NewEnumerator1")
      (bind _doorzroation (Timeline|DoorMechanics Play)
        (:Update
          (Transformation|SetRelativeRotation (Variables|Default|Getdoor_Mesh) (Math|Rotator|MakeRotator 0.0 0.0 _doorzroation) false false))))
    (:NewEnumerator1
      (Variables|Default|SetdoorStatus "NewEnumerator0")
      (Timeline|DoorMechanics Reverse))))

(event EventShowInfo
  (params (HUD :type W%20Overlay%20Object%20Reference))
  (switch Utilities|FlowControl|Switch|SwitchonEN_door-Status (Variables|Default|GetdoorStatus)
    (:NewEnumerator0
      (Default|SetInfoText HUD "drücke [F] zum öffnen"))
    (:NewEnumerator1
      (Default|SetInfoText HUD "drücke [F] zum schließen"))))

(fn ConstructionScript)