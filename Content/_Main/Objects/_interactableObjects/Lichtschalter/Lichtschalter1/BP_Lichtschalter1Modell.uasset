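; Interactable light switch Blueprint that toggles its LED light on and off and shows a German HUD prompt for the current state.
; Interact flips the Lichtstatus enum and sets LED intensity only when IsLichtAn is true; otherwise the prompt reports the power is out.
; Every press, powered or not, replays a timeline from the start to lerp the rocker's pitch, with the same playback direction for both states.
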(event EventInteract
  (params (BP_firstPersonCharacter :type BP%20First%20Person%20Character%20Object%20Reference))
  (bind _led (Variables|Default|GetLED))
  (if (Variables|Default|GetisLichtAn?)
    (switch Utilities|FlowControl|Switch|SwitchonEN_Lichtsalter-Status (Variables|Default|GetLichtstatus)
      (:NewEnumerator0
        (Variables|Default|SetLichtstatus "NewEnumerator1")
        (Rendering|Components|Light|SetIntensity _led 1e+04)
        (bind _lichtschalterbewegung (Timeline|TL_Lichtschalterklick PlayFromStart)
          (:Update
            (Transformation|SetRelativeRotation (Variables|Default|GetLichtschalter1Wipe) (Math|Rotator|MakeRotator 0.0 (Math|Float|Lerp 5.0 -5.0 _lichtschalterbewegung) 0.0) false false))))
      (:NewEnumerator1
        (Variables|Default|SetLichtstatus "NewEnumerator0")
        (Rendering|Components|Light|SetIntensity _led 0.0)
        (Timeline|TL_Lichtschalterklick PlayFromStart)))
    (else
      (Timeline|TL_Lichtschalterklick PlayFromStart))))

(event EventShowInfo
  (params (HUD :type W%20Overlay%20Object%20Reference))
  (if (Variables|Default|GetisLichtAn?)
    (switch Utilities|FlowControl|Switch|SwitchonEN_Lichtsalter-Status (Variables|Default|GetLichtstatus)
      (:NewEnumerator0
        (Default|SetInfoText HUD "drücke [F] um das Licht anzuschalten "))
      (:NewEnumerator1
        (Default|SetInfoText HUD "drücke [F] um das Licht auszuschalten ")))
    (else
      (Default|SetInfoText HUD "Der Strom ist aus!"))))

(fn ConstructionScript)