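; BP_Munitionskiste1 is an interactable ammo crate that the player picks up to restock supplies.
; On Interact it adds pistol and rifle magazines, a medkit and a battery to the BPFirstPersonCharacter's counters, then destroys itself.
; ShowInfo sets a German pickup prompt for the F key on the HUD.
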(event EventInteract
  (params (BP_firstPersonCharacter :type BP%20First%20Person%20Character%20Object%20Reference))
  (Variables|/Game/_Main/_Character/BP_FirstPersonCharacter.BP_FirstPersonCharacter_C|SetPistolMags BP_firstPersonCharacter (+ (Variables|/Game/_Main/_Character/BP_FirstPersonCharacter.BP_FirstPersonCharacter_C|GetPistolMags BP_firstPersonCharacter) 2))
  (Variables|/Game/_Main/_Character/BP_FirstPersonCharacter.BP_FirstPersonCharacter_C|SetRifelMags BP_firstPersonCharacter (+ (Variables|/Game/_Main/_Character/BP_FirstPersonCharacter.BP_FirstPersonCharacter_C|GetRifelMags BP_firstPersonCharacter) 2))
  (Variables|/Game/_Main/_Character/BP_FirstPersonCharacter.BP_FirstPersonCharacter_C|SetMedkitanzahl BP_firstPersonCharacter (+ (Variables|/Game/_Main/_Character/BP_FirstPersonCharacter.BP_FirstPersonCharacter_C|GetMedkitanzahl BP_firstPersonCharacter) 1))
  (Variables|/Game/_Main/_Character/BP_FirstPersonCharacter.BP_FirstPersonCharacter_C|SetBatterieanzahl BP_firstPersonCharacter (+ (Variables|/Game/_Main/_Character/BP_FirstPersonCharacter.BP_FirstPersonCharacter_C|GetBatterieanzahl BP_firstPersonCharacter) 1))
  (Actor|DestroyActor))

(event EventShowInfo
  (params (HUD :type W%20Overlay%20Object%20Reference))
  (Default|SetInfoText HUD "drücke [F] zum Aufsammeln"))

(fn ConstructionScript)